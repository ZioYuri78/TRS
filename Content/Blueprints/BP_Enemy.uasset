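; Enemy ghost with a simple step-based AI that chases the player by line of sight.
; Once woken, it starts on the player controller's moves-queue event and chains timeline-driven 90-degree turns or forward steps up to the controller's move limit.
; Each move line-traces ahead and sideways for the player, turning randomly when blocked.
; Touching the player destroys the ghost if the player is scaled, otherwise kills the player.
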(event `PlayMove`
  ;[1 1 1] Very basic AI
  (if (< (`self.MovesCounter`) (`self.MaxMoves`))
    (bind (_isplayer _distancetohit) (`self.SearchForPlayer` (`self.GetActorForwardVector`) (`self.TraceRange`)))
    (if _isplayer
      (`self.Translate`)
      (elif (> _distancetohit 51.0)
        (bind _isplayer_2 (`self.SearchForPlayer` (`KismetMathLibrary.NegateVector` (`self.GetActorRightVector`)) (`self.TraceRange`)))
        (if _isplayer_2
          (`self.Rotate` "NewEnumerator1")
          (else
            (bind _isplayer_3 (`self.SearchForPlayer` (`self.GetActorRightVector`) (`self.TraceRange`)))
            (if _isplayer_3
              (`self.Rotate` "NewEnumerator0")
              (else
                (`self.Translate`)))))
        (else
          (`self.Rotate` (select `int` (`KismetMathLibrary.RandomInteger` 2) :`0` "NewEnumerator0" :`1` "NewEnumerator1" :!type "/Game/Blueprints/Enums/ETRSOrientation Enum")))))
    (`/Engine/EditorBlueprintResources/StandardMacros.IncrementInt` (`self.MovesCounter`))
    (else
      (set `self.MovesCounter` 0))))

(event `WakeupAI`
  ;[1 1 1] Wake up the AI
  (bind _asbp_player_controller (cast `/Game/Blueprints/BP_PlayerController` (`GameplayStatics.GetPlayerController` 0)))
  (set `self.MaxMoves` (`/Game/Blueprints/BP_PlayerController.MaxMoves` _asbp_player_controller))
  (add `/Game/Blueprints/BP_PlayerController.ED_MovesQueueStarted` _asbp_player_controller (delegate `StartMovements`)))

(event `StartMovements`
  ;[1 1 1] Wake up the AI
  (`self.PlayMove`))

(event `Rotate`
  (params (Orientation :type "/Game/Blueprints/Enums/ETRSOrientation Enum" :default "NewEnumerator0"))
  ;[1 1 1] Rotate
  (switch `/Game/Blueprints/Enums/ETRSOrientation` Orientation
    (:`NewEnumerator0`
      (set `self.TargetRotation` (struct :`Yaw` 90.0)))
    (:`NewEnumerator1`
      (set `self.TargetRotation` (struct :`Yaw` -90.0))))
  (set `self.StartRotation` (`self.K2_GetActorRotation`))
  (bind (_direction _rotate) (`Timeline|TLRotate` :!via `PlayFromStart`)
    (:`Update`
      (`self.K2_SetActorRelativeRotation` (`KismetMathLibrary.RInterpTo` (`self.StartRotation`) (`KismetMathLibrary.ComposeRotators` (`self.StartRotation`) (`self.TargetRotation`)) _rotate (`self.InterSpeed`))))
    (:`Finished`
      (`self.PlayMove`))))

(event `Translate`
  ;[1 1 1] Translate
  (set `self.StartLocation` (`self.K2_GetActorLocation`))
  (bind (_direction _translate) (`Timeline|TLTranslate` :!via `PlayFromStart`)
    (:`Update`
      (`self.K2_SetActorRelativeLocation` (`KismetMathLibrary.VInterpTo` (`self.StartLocation`) (+ (`self.StartLocation`) (* (`self.GetActorForwardVector`) (`self.TranslationRange`))) _translate (`self.InterSpeed`))))
    (:`Finished`
      (`self.PlayMove`))))

(event `self.Capsule.OnComponentBeginOverlap`
  (params (OverlappedComponent :type "PrimitiveComponent Object Reference") (OtherActor :type "Actor Object Reference") (OtherComp :type "PrimitiveComponent Object Reference") (OtherBodyIndex :type Integer) (bFromSweep :type Boolean) (SweepResult :type "HitResult Structure (by ref)"))
  (bind _returnvalue (`GameplayStatics.GetPlayerPawn` 0))
  ;[1 1 1] Manage Overlaps
  (if (== OtherActor _returnvalue)
    (`GameplayStatics.PlaySound2D` (`self.DestroySFX`))
    (`GameplayStatics.SpawnEmitterAtLocation` "/Game/GameJamKit/Effects/Explosions/P_DPW_bot_tank_explo.P_DPW_bot_tank_explo" (`self.K2_GetActorLocation`))
    (`ActorComponent.K2_DestroyComponent` (`self.SM_Ghost`))
    (bind _asbp_player_controller (cast `/Game/Blueprints/BP_PlayerController` (`self.GetController` _returnvalue)))
    (if (`/Game/Blueprints/BP_PlayerController.IsScaled` _asbp_player_controller)
      (`self.K2_DestroyActor`)
      (else
        (bind _asbp_player (cast `/Game/Blueprints/BP_Player` _returnvalue))
        (`/Game/Blueprints/BP_Player.Death` _asbp_player)
        (`KismetSystemLibrary.Delay` 1.0)
        (`self.K2_DestroyActor` _returnvalue)))))

(fn `SearchForPlayer`
  (params (Direction :type "Vector Structure") (Range :type "Float (double-precision)") (DrawDebugType :type "EDrawDebugTrace Enum" :default "None"))
  (returns (IsPlayer :type Boolean) (DistanceToHit :type "Float (double-precision)"))
  (bind _returnvalue (`self.K2_GetActorLocation`))
  (bind _outhit (`KismetSystemLibrary.LineTraceSingle` :`Start` _returnvalue :`End` (+ _returnvalue (* Direction Range)) :`TraceChannel` "TraceTypeQuery1" :`DrawDebugType` DrawDebugType))
  (bind (_bblockinghit _binitialoverlap _time _distance _location _impactpoint _normal _impactnormal _physmat _hitactor) (`GameplayStatics.BreakHitResult` _outhit))
  (return (== (`GameplayStatics.GetObjectClass` _hitactor) "/Game/Blueprints/BP_Player.BP_Player_C") (`KismetMathLibrary.VSize` (- _location (`self.K2_GetActorLocation`)))))

(fn `UserConstructionScript`)