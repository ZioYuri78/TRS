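; BP_2xTranslation is a bonus pickup actor that doubles the player's translation range.
; When the player pawn overlaps its SM_SpeedIcon component, it calls Set2xTranslation on BP_PlayerController, plays a 2D pickup sound and destroys itself.
; The pickup is ignored while the controller's Is2xActive flag is set, so it stays in the level and the bonus does not stack.
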(event `self.SM_SpeedIcon.OnComponentBeginOverlap`
  (params (OverlappedComponent :type "PrimitiveComponent Object Reference") (OtherActor :type "Actor Object Reference") (OtherComp :type "PrimitiveComponent Object Reference") (OtherBodyIndex :type Integer) (bFromSweep :type Boolean) (SweepResult :type "HitResult Structure (by ref)"))
  (bind _returnvalue (`GameplayStatics.GetPlayerPawn` 0))
  (bind _asbp_player_controller (cast `/Game/Blueprints/BP_PlayerController` (`Pawn.GetController` _returnvalue) :!pure true))
  ;[1 1 1] When player pickup the bonus we double the translation range.
  (if (and (== OtherActor _returnvalue) (not (`/Game/Blueprints/BP_PlayerController.Is2xActive` _asbp_player_controller)))
    (`/Game/Blueprints/BP_PlayerController.Set2xTranslation` _asbp_player_controller true)
    (`GameplayStatics.PlaySound2D` (`self.PickUpSound`))
    (`self.K2_DestroyActor`)))

(fn `UserConstructionScript`)