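; BP_Camera is a camera actor that shifts a fixed distance forward or backward along world X when MoveCamera is called.
; The event stores the current location, offsets the target by direction and restarts a timeline.
; Timeline updates set the location through VInterpTo from the stored start, fed by the timeline's DeltaTime output.
; On finish, it calls an EDMovementFinished dispatcher with the target location.
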(event `MoveCamera`
  (params (ISForward :type Boolean))
  ;[1 1 1] Camera movement
  (set `self.StartCameraLocation` (`self.K2_GetActorLocation`))
  (if ISForward
    (set `self.TargetCameraLocation` (+ (`self.StartCameraLocation`) (1100.0 0.0 0.0)))
    (bind (_direction _deltatime) (`Timeline|Timeline_0` :!via `PlayFromStart` :!label _label)
      (:`Update`
        (`self.K2_SetActorLocation` (`KismetMathLibrary.VInterpTo` (`self.StartCameraLocation`) (`self.TargetCameraLocation`) _deltatime (`self.InterpSpeed`))))
      (:`Finished`
        (`self.ED_MovementFinished` (`self.TargetCameraLocation`))))
    (else
      (set `self.TargetCameraLocation` (+ (`self.StartCameraLocation`) (-1100.0 0.0 0.0)))
      (goto _label :!via `PlayFromStart`))))

(fn `UserConstructionScript`)