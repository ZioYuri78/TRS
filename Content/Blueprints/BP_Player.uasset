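; Player pawn that executes translate, 90-degree rotate and half/full scale moves, and reports game over to BP_TRSGameMode when destroyed.
; Timelines interpolate each move and call PlayNextMove on the player controller when finished, except single scale moves.
; A forward trace shortens translations aimed at walls or doors, and overlapping a wall or closed door reverses the movement.
; Death disables collision, removes the mesh and stops all timelines.
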(event `self.ReceiveBeginPlay`
  ;[1 1 1] Bind OnDestroyed at BeginPlay time
  (bind _asbp_player_controller (cast `/Game/Blueprints/BP_PlayerController` (`GameplayStatics.GetPlayerController` 0)))
  (set `self.BP_PlayerController` _asbp_player_controller)
  (add `self.OnDestroyed` (delegate `PlayerDestroyed`)))

(event `self.CapsuleComponent.OnComponentBeginOverlap`
  (params (OverlappedComponent :type "PrimitiveComponent Object Reference") (OtherActor :type "Actor Object Reference") (OtherComp :type "PrimitiveComponent Object Reference") (OtherBodyIndex :type Integer) (bFromSweep :type Boolean) (SweepResult :type "HitResult Structure (by ref)"))
  ;[1 1 1] Mange hit against walls or doors
  (bind _asbp_door (cast `/Game/Blueprints/Environment/DoubleDoors/BP_Door` OtherActor)
    (:`then`
      (if (not (`/Game/Blueprints/Environment/DoubleDoors/BP_Door.IsOpen` _asbp_door))
        (`self.ReverseMovement` :!label _label)))
    (:`CastFailed`
      (cast `/Game/Blueprints/Environment/BP_Wall` OtherActor)
      (goto _label))))

(event `PlayerDestroyed` :!signature `self.OnDestroyed`
  (params (DestroyedActor :type "Actor Object Reference"))
  ;[1 1 1] Bind OnDestroyed at BeginPlay time
  (bind _asbp_trsgame_mode (cast `/Game/Blueprints/Framework/BP_TRSGameMode` (`GameplayStatics.GetGameMode`)))
  (`/Game/Blueprints/Framework/BP_TRSGameMode.GameOver` _asbp_trsgame_mode true))

(event `/Game/Blueprints/Interfaces/BPI_Moves.Translate`
  (params (Range :type "Float (single-precision)"))
  ;[1 1 1] Translate event interface implementation
  (bind _output_get (set `self.StartLocation` (`self.K2_GetActorLocation`)))
  (bind _output_get_2 (set `self.TargetLocation` (+ (`self.StartLocation`) (* (`self.GetActorForwardVector`) Range))))
  (bind (_outhit _returnvalue) (`KismetSystemLibrary.LineTraceSingle` _output_get _output_get_2 "TraceTypeQuery1"))
  (if _returnvalue
    (bind (_bblockinghit _binitialoverlap _time _distance _location _impactpoint _normal _impactnormal _physmat _hitactor) (`GameplayStatics.BreakHitResult` _outhit))
    (if (or (== (`GameplayStatics.GetObjectClass` _hitactor) "/Game/Blueprints/Environment/BP_Wall.BP_Wall_C") (== (`GameplayStatics.GetObjectClass` _hitactor) "/Game/Blueprints/Environment/DoubleDoors/BP_Door.BP_Door_C"))
      (set `self.TargetLocation` (+ (`self.StartLocation`) (* (`self.GetActorForwardVector`) 100.0)))
      (bind (_direction _translate) (`Timeline|TLTranslate` :!via `PlayFromStart` :!label _label_2)
        (:`Update`
          (`self.K2_SetActorRelativeLocation` (`KismetMathLibrary.VInterpTo` (`self.StartLocation`) (`self.TargetLocation`) _translate (`self.InterSpeed`))))
        (:`Finished`
          (`/Game/Blueprints/BP_PlayerController.PlayNextMove` (`self.BP_PlayerController`))))
      (else
        (goto _label_2 :!via `PlayFromStart`)))
    (else
      (goto _label_2 :!via `PlayFromStart`))))

(event `StopTranslation`
  ;[1 1 1] Translate event interface implementation
  (goto _label_2 :!via `Stop`))

(event `ReverseMovement`
  ;[1 1 1] Translate event interface implementation
  (goto _label_2 :!via `Reverse`))

(event `/Game/Blueprints/Interfaces/BPI_Moves.Rotate`
  (params (Orientation :type "/Game/Blueprints/Enums/ETRSOrientation Enum" :default "NewEnumerator0"))
  ;[1 1 1] Rotate event interface implementation
  (switch `/Game/Blueprints/Enums/ETRSOrientation` Orientation
    (:`NewEnumerator0`
      (set `self.TargetRotation` (struct :`Yaw` 90.0)))
    (:`NewEnumerator1`
      (set `self.TargetRotation` (struct :`Yaw` -90.0))))
  (set `self.StartRotation` (`self.K2_GetActorRotation`))
  (bind (_direction _rotate) (`Timeline|TLRotate` :!via `PlayFromStart` :!label _label_3)
    (:`Update`
      (`self.K2_SetActorRelativeRotation` (`KismetMathLibrary.RInterpTo` (`self.StartRotation`) (`KismetMathLibrary.ComposeRotators` (`self.StartRotation`) (`self.TargetRotation`)) _rotate (`self.InterSpeed`))))
    (:`Finished`
      (`/Game/Blueprints/BP_PlayerController.PlayNextMove` (`self.BP_PlayerController`)))))

(event `/Game/Blueprints/Interfaces/BPI_Moves.Scale`
  (params (IsSingleMove :type Boolean))
  (bind _bp_playercontroller (`self.BP_PlayerController`))
  (bind _isscaled (`/Game/Blueprints/BP_PlayerController.IsScaled` _bp_playercontroller))
  ;[1 1 1] Scale event interface implementation
  (if _isscaled
    (set `self.TargetScale` (0.5 0.5 0.5))
    (else
      (set `self.TargetScale` (1.0 1.0 1.0))))
  (set `/Game/Blueprints/BP_PlayerController.IsScaled` (not _isscaled) _bp_playercontroller)
  (set `self.StartScale` (`SceneComponent.K2_GetComponentScale` (`self.StaticMesh`)))
  (bind (_direction _scale) (`Timeline|TLScale` :!via `PlayFromStart` :!label _label_4)
    (:`Update`
      (`SceneComponent.SetRelativeScale3D` (`self.StaticMesh`) (`KismetMathLibrary.VInterpTo` (`self.StartScale`) (`self.TargetScale`) _scale (`self.InterSpeed`))))
    (:`Finished`
      (if (not IsSingleMove)
        (`/Game/Blueprints/BP_PlayerController.PlayNextMove` (`self.BP_PlayerController`))))))

(event `StopRotation`
  ;[1 1 1] Rotate event interface implementation
  (goto _label_3 :!via `Stop`))

(event `StopScale`
  ;[1 1 1] Scale event interface implementation
  (goto _label_4 :!via `Stop`))

(fn `Death`
  (`PrimitiveComponent.SetCollisionEnabled` (`self.CapsuleComponent`) "NoCollision")
  (`ActorComponent.K2_DestroyComponent` (`self.StaticMesh`))
  (`self.StopTranslation`)
  (`self.StopRotation`)
  (`self.StopScale`))

(fn `UserConstructionScript`)