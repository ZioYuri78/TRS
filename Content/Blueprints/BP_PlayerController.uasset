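; Player controller for a turn-based puzzle game where the player queues translate, rotate and scale moves, then plays them on the pawn.
; Key inputs fill a fixed-size move queue and notify listeners through event dispatchers; playback unlocks only when it is full.
; ElaborateQueue disables input and starts PlayNextMove, which pops one move per call.
; An emptied queue re-enables input outside tutorial messages and advances the scale cooldown and timed 2x translation bonus.
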(event `InputAction|Translate`
  (params (Key :type "Key Structure"))
  ;[1 1 1] Keyboard shortcuts
  (:`Pressed`
    (`self.AddMoveToQueue` "NewEnumerator0")))

(event `self.ReceiveBeginPlay`
  ;[1 1 1] Beginplay
  (`KismetSystemLibrary.Delay` 0.2)
  (`WidgetBlueprintLibrary.SetInputMode_GameAndUIEx` self (`/Game/Blueprints/Framework/BP_TRSGameJamKit_InGame_HUD.InGameHUD` (cast `/Game/Blueprints/Framework/BP_TRSGameJamKit_InGame_HUD` (`self.GetHUD`) :!pure true)))
  (set `self.bShowMouseCursor` true))

(event `InputAction|ShowControlsScheme`
  (params (Key :type "Key Structure"))
  ;[1 1 1] Keyboard shortcuts
  (:`Pressed`
    (`self.ED_ShowControlsScheme` "Forward"))
  (:`Released`
    (`self.ED_ShowControlsScheme` "Reverse")))

(event `InputAction|RotateCCW`
  (params (Key :type "Key Structure"))
  ;[1 1 1] Keyboard shortcuts
  (:`Pressed`
    (`self.AddMoveToQueue` "NewEnumerator3")))

(event `InputAction|Scale`
  (params (Key :type "Key Structure"))
  ;[1 1 1] Keyboard shortcuts
  (:`Pressed`
    (if (`self.CanScale`)
      (`self.AddMoveToQueue` "NewEnumerator2")
      (bind _output_get (set `self.CanScale` false))
      (`self.ED_CanScale` _output_get))))

(event `InputAction|Pause` :paused true
  (params (Key :type "Key Structure"))
  ;[1 1 1] Pause the game and show the in game menu
  (:`Pressed`
    (message `/Game/GameJamKit/Blueprints/BP_GameJamKit_HUD_Interface.SetPaused` (`self.GetHUD`) (not (`GameplayStatics.IsGamePaused`)))))

(event `InputAction|RotateCW`
  (params (Key :type "Key Structure"))
  ;[1 1 1] Keyboard shortcuts
  (:`Pressed`
    (`self.AddMoveToQueue` "NewEnumerator1")))

(event `InputAction|DeleteMove`
  (params (Key :type "Key Structure"))
  ;[1 1 1] Keyboard shortcuts
  (:`Pressed`
    (`self.ED_CancelLastMove`)))

(event `InputAction|PlayMoves`
  (params (Key :type "Key Structure"))
  ;[1 1 1] Keyboard shortcuts
  (:`Pressed`
    (if (`self.CanPlayMoves`)
      (`self.ElaborateQueue`))))

(event `ScaleEvent`
  (params (IsSingleMove :type Boolean))
  ;[1 1 1] Scale
  (message `/Game/Blueprints/Interfaces/BPI_Moves.Scale` (`self.K2_GetPawn`) IsSingleMove))

(event `RotateEvent`
  (params (Orientation :type "/Game/Blueprints/Enums/ETRSOrientation Enum" :default "NewEnumerator0"))
  ;[1 1 1] Rotate (fixed 90Degrees CW/CCW)
  (message `/Game/Blueprints/Interfaces/BPI_Moves.Rotate` (`self.K2_GetPawn`) Orientation))

(event `TranslateEvent`
  ;[1 1 1] Translate
  (`GameplayStatics.PlaySound2D` (`self.TranslateSound`))
  (message `/Game/Blueprints/Interfaces/BPI_Moves.Translate` (`self.K2_GetPawn`) (`self.TranslateRange`)))

(fn `AddMoveToQueue`
  (params (Move :type "/Game/Blueprints/Enums/ETRSMoves Enum" :default "NewEnumerator0"))
  (locals (MoveText :type Text))
  (if (< (`KismetArrayLibrary.Array_Length` (`self.MovesQueue`)) (`self.MaxMoves`))
    (`KismetArrayLibrary.Array_Add` (`self.MovesQueue`) Move)
    (`self.ED_MoveAdded` Move)
    (if (== (`KismetArrayLibrary.Array_Length` (`self.MovesQueue`)) (`self.MaxMoves`))
      (set `self.CanPlayMoves` true)
      (`self.ED_QueueIsFull`)
      (return)
      (else
        (set `self.CanPlayMoves` false)
        (return)))
    (else
      (return))))

(fn `ClearQueue`
  (`KismetArrayLibrary.Array_Clear` (`self.MovesQueue`)))

(fn `ElaborateQueue`
  (`self.DisableInput` self)
  (`self.PlayNextMove`)
  (`self.ED_MovesQueueStarted`))

(fn `PlayNextMove`
  (bind _scaleturncounter (`self.ScaleTurnCounter`))
  (if (`KismetArrayLibrary.Array_IsValidIndex` (`self.MovesQueue`))
    (switch `/Game/Blueprints/Enums/ETRSMoves` (`|GetArrayItem` (`self.MovesQueue`))
      (:`NewEnumerator0`
        (`self.TranslateEvent`))
      (:`NewEnumerator1`
        (`self.RotateEvent` "NewEnumerator0"))
      (:`NewEnumerator3`
        (`self.RotateEvent` "NewEnumerator1"))
      (:`NewEnumerator2`
        (`self.ScaleEvent` false)))
    (`self.ED_MoveRemoved`)
    (`KismetArrayLibrary.Array_Remove` (`self.MovesQueue`))
    (return)
    (else
      (set `self.CanPlayMoves` false)
      (`self.ED_QueueIsEmpty`)
      (if (`self.Is2xActive`)
        (set `self.TranslateRange` 200.0)
        (`/Engine/EditorBlueprintResources/StandardMacros.IsValid` (`self.TranslateSound`)
          (:`Is Valid`
            _)
          (:`Is Not Valid`
            (set `self.TranslateSound` "/Game/SFX/SFX_2xTranslate_Cue.SFX_2xTranslate_Cue")))
        (if (>= (`self.2xTurnCounter`) (`self.2xCooldown`))
          (set `self.2xTurnCounter` 0)
          (`self.Set2xTranslation` false)
          (else
            (`/Engine/EditorBlueprintResources/StandardMacros.IncrementInt` (`self.2xTurnCounter`)
              (:`  `
                _)))))
      (if (`self.IsScaled`)
        (`self.ScaleEvent` true))
      (if (not (`/Game/Blueprints/Framework/BP_TRSGameMode.IsTutorialMsgActive` (cast `/Game/Blueprints/Framework/BP_TRSGameMode` (`GameplayStatics.GetGameMode`) :!pure true)))
        (`self.EnableInput` self))
      (if (`self.CanScale`)
        _
        (elif (>= _scaleturncounter (`self.ScaleCooldown`))
          (set `self.ScaleTurnCounter` 0)
          (bind _output_get (set `self.CanScale` true))
          (`self.ED_CanScale` _output_get)
          (else
            (`/Engine/EditorBlueprintResources/StandardMacros.IncrementInt` _scaleturncounter
              (:`  `
                _)))))
      (return))))

(fn `RemoveLastMove`
  (returns (LastIndex :type Integer))
  (locals (LocalLastIndex :type Integer :default 0))
  (bind _movesqueue (`self.MovesQueue`))
  (bind _locallastindex (`local.LocalLastIndex`))
  (set `self.CanPlayMoves` false)
  (bind _output_get (set `local.LocalLastIndex` (`KismetArrayLibrary.Array_LastIndex` _movesqueue)))
  (if (`|EnumEquality` (`|GetArrayItem` _movesqueue _output_get) "NewEnumerator2")
    (bind _output_get_2 (set `self.CanScale` true))
    (`self.ED_CanScale` _output_get_2))
  (`KismetArrayLibrary.Array_Remove` (`self.MovesQueue`) _locallastindex)
  (return _locallastindex))

(fn `Set2xTranslation`
  (params (Is2xActive :type Boolean))
  (if Is2xActive
    (set `self.Is2xActive` true)
    (`self.ED_2xBonus` true)
    (else
      (set `self.Is2xActive` false)
      (set `self.TranslateRange` 100.0)
      (set `self.TranslateSound` null)
      (`self.ED_2xBonus` false)))
  (return))

(fn `UserConstructionScript`)