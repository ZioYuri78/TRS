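; BP_TRSGameMode is the game mode that coordinates stage transitions, game over, coin updates and tutorial messaging.
; On BeginPlay it restores goal coins and level name from saved data in BP_GameInstance and binds to BP_Camera's movement-finished event to save the camera location.
; GameOver shows the HUD win/lose message and returns the view to the camera, while small functions relay coin and tutorial changes through event dispatchers.
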(event `self.ReceiveBeginPlay`
  ;[1 1 1] On BeginPlay we look if we have saved data to display the correct level name and number of goal coins, also we save the game at the end of camera movement (transition between levels).
  (bind _asbp_game_instance (cast `/Game/Blueprints/Framework/BP_GameInstance` (`GameplayStatics.GetGameInstance`)))
  (bind _output_get (set `self.BP_GameInstance` _asbp_game_instance))
  (bind _return_value (`/Game/Blueprints/Framework/BP_GameInstance.IsDataAvailable` _output_get))
  (if _return_value
    (bind (_respawntransform _cameralocation _goalcoins _levelname) (`/Game/Blueprints/Framework/BP_GameInstance.GetRespawnData` _output_get))
    (`self.ED_GoalCoinsUpdate` _goalcoins _levelname))
  (bind _outactors (`GameplayStatics.GetAllActorsOfClass` "/Game/Blueprints/BP_Camera.BP_Camera_C"))
  (bind _output_get_2 (set `self.BP_Camera` (`|GetArrayItem` _outactors)))
  (add `/Game/Blueprints/BP_Camera.ED_MovementFinished` _output_get_2 (delegate `SaveCameraLocation`)))

(event `SaveCameraLocation`
  (params (CameraLocation :type "Vector Structure"))
  (bind _bp_gameinstance (`self.BP_GameInstance`))
  ;[1 1 1] On BeginPlay we look if we have saved data to display the correct level name and number of goal coins, also we save the game at the end of camera movement (transition between levels).
  (`/Game/Blueprints/Framework/BP_GameInstance.SetCameraLocation` _bp_gameinstance CameraLocation)
  (`/Game/Blueprints/Framework/BP_GameInstance.SaveData` _bp_gameinstance))

(event `GameOver`
  (params (IsGameOver :type Boolean))
  (bind _returnvalue (`GameplayStatics.GetPlayerController` 0))
  ;[1 1 1] Show game over widget, and we set again the BP_Camera as view target, that because player will be destroyed in any game over condition (win/lost) and unpossesed by the player controller.
  (message `/Game/GameJamKit/Blueprints/BP_GameJamKit_HUD_Interface.ShowGameOver` (`PlayerController.GetHUD` _returnvalue) (select `bool` IsGameOver :`false` (`self.YouWon`) :`true` (`self.OhNo`)) IsGameOver)
  (`PlayerController.SetViewTargetWithBlend` _returnvalue (`self.BP_Camera`) 0.0 "VTBlend_Linear" 0.0 false))

(event `NextStage`
  ;[1 1 1] Move the camera to the next stage
  (`/Game/Blueprints/BP_Camera.MoveCamera` (`self.BP_Camera`) true))

(fn `CoinsAdded`
  (params (Coins :type Integer))
  (`self.ED_CoinsAdded` Coins))

(fn `GoalCoinsUpdate`
  (params (Coins :type Integer) (LevelName :type Name))
  (`self.ED_GoalCoinsUpdate` Coins LevelName))

(fn `StartTutorial`
  (params (DoTutorial :type Boolean))
  (`self.ED_TutorialAnswer` DoTutorial))

(fn `TutorialMessage`
  (params (Message :type Text))
  (`self.ED_TutorialMessage` Message)
  (set `self.IsTutorialMsgActive` true))

(fn `UserConstructionScript`)